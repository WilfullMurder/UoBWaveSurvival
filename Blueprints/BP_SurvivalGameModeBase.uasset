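; Survival game mode that spawns bots and awards score for kills.
; SpawnNewBot runs the EQS_FindSpawnLoc query in single-result mode and, on success, spawns a BP_SimpleBot at the returned location with a debug sphere.
; On BeginPlay it binds to OnActorKilled, adding a point to the killer pawn's SurvivalPlayerState and printing the score.
; Nothing in this graph calls SpawnNewBot, and Tick is unused.
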(event `self.SpawnNewBot`
  (bind _returnvalue (`EnvQueryManager.RunEQSQuery` "/Game/Blueprints/NPC/AI/EQS/EQS_FindSpawnLoc.EQS_FindSpawnLoc" self "SingleResult"))
  (add `EnvQueryInstanceBlueprintWrapper.OnQueryFinishedEvent` _returnvalue (delegate `OnQueryFinishedEvent`)))

(event `OnQueryFinishedEvent`
  (params (QueryInstance :type "EnvQueryInstanceBlueprintWrapper Object Reference") (QueryStatus :type "EEnvQueryStatus Enum" :default "Processing"))
  (switch `EEnvQueryStatus` QueryStatus
    (:`Success`
      (bind _resultlocations (`EnvQueryInstanceBlueprintWrapper.GetQueryResultsAsLocations` QueryInstance))
      (for _array_element _resultlocations
        (`KismetSystemLibrary.DrawDebugSphere` _array_element 50.0 12 (struct :`R` 0.348958 :`B` 0.225345 :`A` 1.0) 2.0 1.0)
        (`|SpawnActorFromClass` "/Game/Blueprints/NPC/SimpleBots/BP_SimpleBot.BP_SimpleBot_C" (`KismetMathLibrary.MakeTransform` _array_element) "AdjustIfPossibleButAlwaysSpawn" "OverrideRootScale" null null)))))

(event `self.ReceiveBeginPlay`
  (add `self.OnActorKilled` (delegate `OnActorKilledEvent`)))

(event `OnActorKilledEvent` :!signature `self.OnActorKilled`
  (params (VictimActor :type "Actor Object Reference") (KillerActor :type "Actor Object Reference") (KillerController :type "Controller Object Reference"))
  (bind _aspawn (cast `Pawn` KillerActor))
  (bind _assurvival_player_state (cast `SurvivalPlayerState` (`Pawn.PlayerState` _aspawn)))
  (`SurvivalPlayerState.AddScore` _assurvival_player_state 1.0)
  (`KismetSystemLibrary.PrintString` (`KismetStringLibrary.Conv_DoubleToString` (`PlayerState.Score` _assurvival_player_state))))

(fn `UserConstructionScript`)