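; Healing-over-time powerup pickup that restores a fixed amount of health to the actor that activated it on each powerup tick.
; Activation stores the target, and each tick calls Heal on that target's HealthComponent if it has one.
; On expiry it asks the target, cast to BP_SurvivalCharacter, to destroy it on the server.
; From BeginPlay, a short looping timer randomly tumbles the mesh, then clears itself after about a second.
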(event `self.ReceiveBeginPlay`
  (set `self.LoopCount` 0)
  (bind _returnvalue (`KismetSystemLibrary.K2_SetTimerDelegate` (delegate `HandleSpinObject`) 0.1 true))
  (set `self.TH_SpinObject` _returnvalue))

(event `HandleSpinObject`
  (bind _returnvalue (`KismetMathLibrary.RandomFloatInRange` -360.0 360.0))
  (`SceneComponent.K2_SetRelativeRotation` (`self.Mesh`) (`KismetMathLibrary.MakeRotator` (+ (.roll (`SceneComponent.RelativeRotation` (`self.Mesh`))) _returnvalue) (+ (.pitch (`SceneComponent.RelativeRotation` (`self.Mesh`))) _returnvalue) (+ (.yaw (`SceneComponent.RelativeRotation` (`self.Mesh`))) _returnvalue)) false false)
  (bind _output_get (set `self.LoopCount` (+ (`self.LoopCount`) 1)))
  (if (> _output_get 10)
    (`KismetSystemLibrary.K2_ClearAndInvalidateTimerHandle` (`self.TH_SpinObject`))))

(event `self.OnPowerupTicked`
  (bind _returnvalue (`self.GetComponentByClass` (`self.PlayerTarget`) "/Script/Survival.HealthComponent"))
  (`/Engine/EditorBlueprintResources/StandardMacros.IsValid` _returnvalue
    (:`Is Valid`
      (`HealthComponent.Heal` _returnvalue 5.0))))

(event `self.OnActivated`
  (params (ActiveFor :type "Actor Object Reference"))
  (set `self.PlayerTarget` ActiveFor))

(event `self.OnExpired`
  (bind _asbp_survival_character (cast `/Game/Blueprints/PlayerCharacter/BP_SurvivalCharacter` (`self.PlayerTarget`)))
  (`/Engine/EditorBlueprintResources/StandardMacros.IsValid` _asbp_survival_character
    (:`Is Valid`
      (`/Game/Blueprints/PlayerCharacter/BP_SurvivalCharacter.DestroyActorOnServer` _asbp_survival_character self))))

(fn `UserConstructionScript`)