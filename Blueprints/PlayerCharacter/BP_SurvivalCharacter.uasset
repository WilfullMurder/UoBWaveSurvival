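; Player character Blueprint for survival gameplay that sets up the local HUD and provides a way to destroy actors.
; On BeginPlay, only the locally controlled character creates crosshair and health indicator widgets and adds them to the viewport.
; DestroyActorOnServer forwards a target to DestroyActorOnClient, which destroys it if valid; the event names suggest a server-to-client relay.
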(event `self.ReceiveBeginPlay`
  (if (`self.IsLocallyControlled`)
    (`|ExecutionSequence`
      (:`then_0`
        (bind _returnvalue (`|CreateWidget` "/Game/Blueprints/Weapons/WBP_Crosshair.WBP_Crosshair_C"))
        (`UserWidget.AddToViewport` _returnvalue 0))
      (:`then_1`
        (bind _returnvalue_2 (`|CreateWidget` "/Game/Blueprints/UI/WBP_HealthIndicator.WBP_HealthIndicator_C"))
        (`UserWidget.AddToViewport` _returnvalue_2 0)))))

(event `DestroyActorOnServer`
  (params (TargetActor :type "Actor Object Reference"))
  (`self.DestroyActorOnClient` TargetActor))

(event `DestroyActorOnClient`
  (params (TargetActor :type "Actor Object Reference"))
  (`/Engine/EditorBlueprintResources/StandardMacros.IsValid` TargetActor
    (:`Is Valid`
      (`self.K2_DestroyActor` TargetActor))))

(fn `UserConstructionScript`)