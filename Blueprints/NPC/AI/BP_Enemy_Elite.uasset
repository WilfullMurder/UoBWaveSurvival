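; Elite enemy Blueprint that drops a pickup when its health runs out.
; On BeginPlay it binds to its HealthComponent's health-changed event.
; When health is zero or below and the component's owner is an elite enemy, it spawns a BP_PickupActor slightly raised and randomly offset horizontally from that owner.
; The spawn always ignores collision, and no guard in this graph prevents repeat drops on later health changes.
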(event `self.ReceiveBeginPlay`
  (add `HealthComponent.OnHealthChanged` (`self.HealthComponent`) (delegate `OnHealthChangedEvent`)))

(event `OnHealthChangedEvent`
  (params (OwningHealthComp :type "HealthComponent Object Reference") (Health :type "Float (double-precision)") (HealthDelta :type "Float (double-precision)") (DamageType :type "DamageType Object Reference") (InstigatedBy :type "Controller Object Reference") (DamageCauser :type "Actor Object Reference"))
  (bind _returnvalue (`ActorComponent.GetOwner` OwningHealthComp))
  (`/Engine/EditorBlueprintResources/StandardMacros.IsValid` OwningHealthComp
    (:`Is Valid`
      (if (<= Health 0.0)
        (bind _asbp_enemy_elite (cast `/Blueprints/NPC/AI/BP_Enemy_Elite` _returnvalue))
        (`/Engine/EditorBlueprintResources/StandardMacros.IsValid` _asbp_enemy_elite
          (:`Is Valid`
            (`|SpawnActorFromClass` "/Game/Blueprints/Pickups/BP_PickupActor.BP_PickupActor_C" (`KismetMathLibrary.MakeTransform` (+ (.location (`self.GetTransform` _returnvalue)) (`KismetMathLibrary.MakeVector` (`KismetMathLibrary.RandomFloatInRange` (`KismetMathLibrary.RandomFloatInRange` -300.0 -150.0) (`KismetMathLibrary.RandomFloatInRange` 150.0 300.0)) (`KismetMathLibrary.RandomFloatInRange` (`KismetMathLibrary.RandomFloatInRange` -300.0 -150.0) (`KismetMathLibrary.RandomFloatInRange` 150.0 300.0)) 50.0))) "AlwaysSpawn" "OverrideRootScale" null null)))))))

(event `self.ReceiveTick`
  (params (DeltaSeconds :type "Float (single-precision)")))

(fn `UserConstructionScript`)